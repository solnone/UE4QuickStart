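; BP_Cube is a cube actor whose color animates to a requested value through its ChangeColor event.
; BeginPlay creates a dynamic material instance from M_BaseColor on VisualMesh and stores its initial Color parameter.
; ChangeColor ignores calls while TimelineColor plays, otherwise it runs the timeline to lerp Color from that stored value to the new one.
; The stored color is never updated, so every transition starts from the original color.
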(event `self.ReceiveBeginPlay`
  (bind _returnvalue (`PrimitiveComponent.CreateDynamicMaterialInstance` (`self.VisualMesh`) 0 "/Game/Materials/M_BaseColor.M_BaseColor" "None"))
  (bind _output_get (set `self.Material` _returnvalue))
  (bind _returnvalue_2 (`MaterialInstanceDynamic.K2_GetVectorParameterValue` _output_get "Color"))
  (set `self.KeepColor` _returnvalue_2))

(event `ChangeColor`
  (params (Value :type "LinearColor Structure"))
  (if (not (`TimelineComponent.IsPlaying` (`self.TimelineColor`)))
    (set `self.NewColor` Value)
    (bind (_direction _color) (`Timeline|TimelineColor` :!via `PlayFromStart`)
      (:`Update`
        (`MaterialInstanceDynamic.SetVectorParameterValue` (`self.Material`) "Color" (`KismetMathLibrary.LinearColorLerp` (`self.KeepColor`) (`self.NewColor`) _color))))))

(fn `UserConstructionScript`)